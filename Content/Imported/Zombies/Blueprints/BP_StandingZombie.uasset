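; BP_StandingZombie is a zombie enemy that detects the first-person player and punches them at close range.
; PawnSensing sets a "seen player" Blackboard flag on its AI controller when it spots the player.
; AttackPlayer runs a short forward sphere trace for pawns and, on hitting the player, plays a left-punch montage, applies damage immediately and prints a leftover on-screen string.
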(event OnSeePawn(PawnSensing)
  (params (Pawn :type Pawn%20Object%20Reference))
  (Utilities|Casting|CastToBP_FirstPersonCharacter Pawn)
  (AI|Components|Blackboard|SetValueasBool (AI|GetBlackboard (AI|GetAIController self)) (Utilities|Name|MakeLiteralName "hasSeenPlayer?") true))

(event Custom|Attack%20Player
  (bind _returnvalue (Transformation|GetActorLocation))
  (bind (_outhit _returnvalue_2) (Collision|SphereTraceForObjects _returnvalue (+ _returnvalue (* (Math|Vector|GetForwardVector (Transformation|GetActorRotation)) 2.5e+02)) 15.0 (Utilities|Array|MakeArray "ObjectTypeQuery3") false 0 "None"))
  (if _returnvalue_2
    (Utilities|Casting|CastToBP_FirstPersonCharacter (.HitActor (Collision|BreakHitResult _outhit)))
    (Animation|PlayAnimMontage "/Game/Imported/Zombies/Animations/StandingZombie2/AM_LeftPunch.AM_LeftPunch" 1.0 "None")
    (Game|Damage|ApplyDamage (.HitActor (Collision|BreakHitResult _outhit)) 1e+01 0 0)
    (Development|PrintString "James is gay")))

(fn ConstructionScript)