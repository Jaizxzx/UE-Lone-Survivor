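; Spawner actor that populates the area around itself with standing zombies when play begins.
; A fast looping timer spawns BP_StandingZombie actors at random reachable navmesh points within a wide radius, storing each reference in an array.
; Once a counter reaches its fixed cap, spawning stops and the timer handle is invalidated, though the timer itself is never cleared.
; A DestroySpawnedZombies event destroys every stored zombie, printing a debug message.
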(event Custom|Destroy%20Spawned%20Zombies
  (for _array_element (Variables|Default|GetZombie_Refs)
    (Actor|DestroyActor _array_element)
    (Development|PrintString "Destroy zombies called")))

(event Custom|Spawn%20Zombie
  (if (< (Variables|Default|GetI) 50)
    (bind _returnvalue (Game|SpawnActorfromClass "/Game/Imported/Zombies/Blueprints/BP_StandingZombie.BP_StandingZombie_C" (Math|Transform|MakeTransform (.RandomLocation (AI|Navigation|GetRandomReachablePointinRadius (Transformation|GetActorLocation) 9e+03 0 0)) "0, 0, 0" "1.000000,1.000000,1.000000") "Undefined" "MultiplyWithRoot" 0 0))
    (Utilities|Array|Add (Variables|Default|GetZombie_Refs) _returnvalue)
    (bind _result (Math|Integer|IncrementInt (Variables|Default|GetI))
      (:%20%20
        (Variables|Default|SetI _result)))
    (else
      (Utilities|Time|InvalidateTimerHandle (Variables|Default|GetTimer%20Handle)))))

(event EventBeginPlay
  (bind _returnvalue (Utilities|Time|SetTimerbyEvent (delegate Custom|Spawn%20Zombie) 0.2 true))
  (Variables|Default|SetTimer%20Handle _returnvalue))

(fn ConstructionScript)